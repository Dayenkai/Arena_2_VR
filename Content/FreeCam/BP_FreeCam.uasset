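; Free-flying cinematic camera pawn whose CineCamera lens settings are adjusted live through hotkeys.
; Axis inputs drive movement, while mouse look only works while the "<" key is held to set CamCanMove.
; Modified mouse-wheel keys step manual focus distance and focal length, and keypad keys adjust aperture and switch filmback presets.
; On BeginPlay it adds a W_CamInfo widget to the viewport, passing itself as the camera reference.
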(event EventBeginPlay
  (bind _returnvalue (UserInterface|CreateWidget "/Game/FreeCam/ATH/W_CamInfo.W_CamInfo_C" 0 self))
  (UserInterface|Viewport|AddtoViewport _returnvalue 0))

(event Input|AxisEvents|InputAxisMoveForward
  (params (AxisValue :type Float%20%28single-precision%29))
  ;[1 1 1] Movement
  (Class|DefaultPawn|MoveForward AxisValue))

(event Input|AxisEvents|InputAxisMoveRIght
  (params (AxisValue :type Float%20%28single-precision%29))
  ;[1 1 1] Movement
  (Class|DefaultPawn|MoveRight AxisValue))

(event Input|AxisEvents|InputAxisMoveUp
  (params (AxisValue :type Float%20%28single-precision%29))
  ;[1 1 1] Movement
  (Class|DefaultPawn|MoveUpWorld AxisValue))

(event Input|AxisEvents|InputAxisMouseX
  (params (AxisValue :type Float%20%28single-precision%29))
  ;[1 1 1] Movement
  (if (Variables|Default|GetCamCanMove?)
    (Pawn|Input|AddControllerYawInput AxisValue)))

(event Input|AxisEvents|InputAxisMouseY
  (params (AxisValue :type Float%20%28single-precision%29))
  ;[1 1 1] Movement
  (if (Variables|Default|GetCamCanMove?)
    (Pawn|Input|AddControllerPitchInput AxisValue)))

(event Input|KeyboardEvents|<
  (params (Key :type Key%20Structure))
  ;[1 1 1] Movement
  (:Pressed
    (Variables|Default|SetCamCanMove? true))
  (:Released
    (Variables|Default|SetCamCanMove? false)))

(event Input|KeyboardEvents|CtrlNumPadZero
  (params (Key :type Key%20Structure))
  ;[1 1 1] FilmBack Settings
  (:Pressed
    (Variables|/Script/CinematicCamera.CineCameraComponent|SetFilmbackSettings (Variables|Default|GetCineCamera) (Variables|Default|Get16_9%20DSLR%20Film))))

(event Input|KeyboardEvents|AltNumPadZero
  (params (Key :type Key%20Structure))
  ;[1 1 1] FilmBack Settings
  (:Pressed
    (Variables|/Script/CinematicCamera.CineCameraComponent|SetFilmbackSettings (Variables|Default|GetCineCamera) (Variables|Default|Get16_9%20DSLR%20Digital%20Film))))

(event Input|KeyboardEvents|NumPadTwo
  (params (Key :type Key%20Structure))
  ;[1 1 1] FilmBack Settings
  (:Pressed
    (Variables|/Script/CinematicCamera.CineCameraComponent|SetFilmbackSettings (Variables|Default|GetCineCamera) (Variables|Default|Get35%20mm%20Academy))))

(event Input|KeyboardEvents|CtrlNumPadTwo
  (params (Key :type Key%20Structure))
  ;[1 1 1] FilmBack Settings
  (:Pressed
    (Variables|/Script/CinematicCamera.CineCameraComponent|SetFilmbackSettings (Variables|Default|GetCineCamera) (Variables|Default|Get35%20mm%20Full%20Aperture))))

(event Input|KeyboardEvents|AltNumPadTwo
  (params (Key :type Key%20Structure))
  ;[1 1 1] FilmBack Settings
  (:Pressed
    (Variables|/Script/CinematicCamera.CineCameraComponent|SetFilmbackSettings (Variables|Default|GetCineCamera) (Variables|Default|Get35%20mm%20Vista%20Vision))))

(event Input|KeyboardEvents|AltNumPadThree
  (params (Key :type Key%20Structure))
  ;[1 1 1] FilmBack Settings
  (:Pressed
    (Variables|/Script/CinematicCamera.CineCameraComponent|SetFilmbackSettings (Variables|Default|GetCineCamera) (Variables|Default|GetFull%20Frame%20DSLR))))

(event Input|MouseEvents|AltShiftMouseWheelUp
  (params (Key :type Key%20Structure))
  (bind _cinecamera (Variables|Default|GetCineCamera))
  ;[1 1 1] Focus / Mise au Point
  (:Pressed
    (Variables|/Script/CinematicCamera.CineCameraComponent|SetFocusSettings _cinecamera (Utilities|Struct|MakeCameraFocusSettings "Manual" (+ (Variables|/Script/CinematicCamera.CineCameraComponent|GetCurrentFocusDistance _cinecamera) 1e+01) "(ActorToTrack=None,RelativeOffset=(X=0.000000,Y=0.000000,Z=0.000000))" false 8.0 0.0))))

(event Input|MouseEvents|AltShiftMouseWheelDown
  (params (Key :type Key%20Structure))
  (bind _cinecamera (Variables|Default|GetCineCamera))
  ;[1 1 1] Focus / Mise au Point
  (:Pressed
    (Variables|/Script/CinematicCamera.CineCameraComponent|SetFocusSettings _cinecamera (Utilities|Struct|MakeCameraFocusSettings "Manual" (- (Variables|/Script/CinematicCamera.CineCameraComponent|GetCurrentFocusDistance _cinecamera) 1e+01) "(ActorToTrack=None,RelativeOffset=(X=0.000000,Y=0.000000,Z=0.000000))" false 8.0 0.0))))

(event Input|MouseEvents|MiddleMouseButton
  (params (Key :type Key%20Structure))
  ;[1 1 1] Focal Lenght, Zoom
  (:Pressed
    (Variables|/Script/CinematicCamera.CineCameraComponent|SetCurrentFocalLength (Variables|Default|GetCineCamera) 35.0)))

(event Input|KeyboardEvents|AltAdd
  (params (Key :type Key%20Structure))
  ;[1 1 1] Apertue
  (:Pressed
    (Variables|/Script/CinematicCamera.CineCameraComponent|SetCurrentAperture (Variables|Default|GetCineCamera) 2.8)))

(event Input|KeyboardEvents|CtrlAltNumPadThree
  (params (Key :type Key%20Structure))
  ;[1 1 1] FilmBack Settings
  (:Pressed
    (Variables|/Script/CinematicCamera.CineCameraComponent|SetFilmbackSettings (Variables|Default|GetCineCamera) (Variables|Default|GetMicro%20Four%20Thirds))))

(event Input|KeyboardEvents|CtrlSubtract
  (params (Key :type Key%20Structure))
  (bind _cinecamera (Variables|Default|GetCineCamera))
  ;[1 1 1] Apertue
  (:Pressed
    (Variables|/Script/CinematicCamera.CineCameraComponent|SetCurrentAperture _cinecamera (- (Variables|/Script/CinematicCamera.CineCameraComponent|GetCurrentAperture _cinecamera) 0.5))))

(event Input|KeyboardEvents|Add
  (params (Key :type Key%20Structure))
  (bind _cinecamera (Variables|Default|GetCineCamera))
  ;[1 1 1] Apertue
  (:Pressed
    (Variables|/Script/CinematicCamera.CineCameraComponent|SetCurrentAperture _cinecamera (+ (Variables|/Script/CinematicCamera.CineCameraComponent|GetCurrentAperture _cinecamera) 0.1))))

(event Input|KeyboardEvents|Subtract
  (params (Key :type Key%20Structure))
  (bind _cinecamera (Variables|Default|GetCineCamera))
  ;[1 1 1] Apertue
  (:Pressed
    (Variables|/Script/CinematicCamera.CineCameraComponent|SetCurrentAperture _cinecamera (- (Variables|/Script/CinematicCamera.CineCameraComponent|GetCurrentAperture _cinecamera) 0.1))))

(event Input|KeyboardEvents|CtrlAdd
  (params (Key :type Key%20Structure))
  (bind _cinecamera (Variables|Default|GetCineCamera))
  ;[1 1 1] Apertue
  (:Pressed
    (Variables|/Script/CinematicCamera.CineCameraComponent|SetCurrentAperture _cinecamera (+ (Variables|/Script/CinematicCamera.CineCameraComponent|GetCurrentAperture _cinecamera) 0.5))))

(event Input|MouseEvents|CtrlMouseWheelUp
  (params (Key :type Key%20Structure))
  (bind _cinecamera (Variables|Default|GetCineCamera))
  ;[1 1 1] Focal Lenght, Zoom
  (:Pressed
    (Variables|/Script/CinematicCamera.CineCameraComponent|SetCurrentFocalLength _cinecamera (+ (Variables|/Script/CinematicCamera.CineCameraComponent|GetCurrentFocalLength _cinecamera) 1.0))))

(event Input|MouseEvents|CtrlMouseWheelDown
  (params (Key :type Key%20Structure))
  (bind _cinecamera (Variables|Default|GetCineCamera))
  ;[1 1 1] Focal Lenght, Zoom
  (:Pressed
    (Variables|/Script/CinematicCamera.CineCameraComponent|SetCurrentFocalLength _cinecamera (- (Variables|/Script/CinematicCamera.CineCameraComponent|GetCurrentFocalLength _cinecamera) 1.0))))

(event Input|MouseEvents|AltMouseWheelUp
  (params (Key :type Key%20Structure))
  (bind _cinecamera (Variables|Default|GetCineCamera))
  ;[1 1 1] Focus / Mise au Point
  (:Pressed
    (Variables|/Script/CinematicCamera.CineCameraComponent|SetFocusSettings _cinecamera (Utilities|Struct|MakeCameraFocusSettings "Manual" (+ (Variables|/Script/CinematicCamera.CineCameraComponent|GetCurrentFocusDistance _cinecamera) 1e+02) "(ActorToTrack=None,RelativeOffset=(X=0.000000,Y=0.000000,Z=0.000000))" false 8.0 0.0))))

(event Input|MouseEvents|AltMouseWheelDown
  (params (Key :type Key%20Structure))
  (bind _cinecamera (Variables|Default|GetCineCamera))
  ;[1 1 1] Focus / Mise au Point
  (:Pressed
    (Variables|/Script/CinematicCamera.CineCameraComponent|SetFocusSettings _cinecamera (Utilities|Struct|MakeCameraFocusSettings "Manual" (- (Variables|/Script/CinematicCamera.CineCameraComponent|GetCurrentFocusDistance _cinecamera) 1e+02) "(ActorToTrack=None,RelativeOffset=(X=0.000000,Y=0.000000,Z=0.000000))" false 8.0 0.0))))

(event Input|KeyboardEvents|NumPadThree
  (params (Key :type Key%20Structure))
  ;[1 1 1] FilmBack Settings
  (:Pressed
    (Variables|/Script/CinematicCamera.CineCameraComponent|SetFilmbackSettings (Variables|Default|GetCineCamera) (Variables|Default|GetIMAX))))

(event Input|KeyboardEvents|NumPadNine
  (params (Key :type Key%20Structure))
  ;[1 1 1] FilmBack Settings
  (:Pressed
    (Variables|/Script/CinematicCamera.CineCameraComponent|SetFilmbackSettings (Variables|Default|GetCineCamera) (Variables|Default|Get16_9%20DSLR))))

(event Input|KeyboardEvents|CtrlNumPadThree
  (params (Key :type Key%20Structure))
  ;[1 1 1] FilmBack Settings
  (:Pressed
    (Variables|/Script/CinematicCamera.CineCameraComponent|SetFilmbackSettings (Variables|Default|GetCineCamera) (Variables|Default|GetAPS-C))))

(event Input|KeyboardEvents|NumPadOne
  (params (Key :type Key%20Structure))
  ;[1 1 1] FilmBack Settings
  (:Pressed
    (Variables|/Script/CinematicCamera.CineCameraComponent|SetFilmbackSettings (Variables|Default|GetCineCamera) (Variables|Default|Get16_9%20DSLR%20Super%208))))

(event Input|KeyboardEvents|CtrlNumPadOne
  (params (Key :type Key%20Structure))
  ;[1 1 1] FilmBack Settings
  (:Pressed
    (Variables|/Script/CinematicCamera.CineCameraComponent|SetFilmbackSettings (Variables|Default|GetCineCamera) (Variables|Default|Get16_9%20DSLR%20Super%2016))))

(event Input|KeyboardEvents|AltNumPadOne
  (params (Key :type Key%20Structure))
  ;[1 1 1] FilmBack Settings
  (:Pressed
    (Variables|/Script/CinematicCamera.CineCameraComponent|SetFilmbackSettings (Variables|Default|GetCineCamera) (Variables|Default|Get16_9%20DSLR%20Super%2035))))

(event Input|KeyboardEvents|NumPadZero
  (params (Key :type Key%20Structure))
  ;[1 1 1] FilmBack Settings
  (:Pressed
    (Variables|/Script/CinematicCamera.CineCameraComponent|SetFilmbackSettings (Variables|Default|GetCineCamera) (Variables|Default|Get16_9%20DSLR))))

(fn ConstructionScript)