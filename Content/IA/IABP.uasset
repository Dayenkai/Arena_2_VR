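; Melee AI enemy character that chases the player and punches at close range, with health, armor and a HUD widget.
; AIMoveTo on Tick and a delayed SeekPlayer loop drive pursuit, while a looping timer checks distance to trigger random attack montages.
; Fist overlaps and sphere traces apply damage, currently zero for every attack.
; Heavier hits play a stagger montage, and depleted health plays a KO.
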(event OnComponentBeginOverlap(LeftFist)
  (params (OverlappedComponent :type Primitive%20Component%20Object%20Reference) (OtherActor :type Actor%20Object%20Reference) (OtherComp :type Primitive%20Component%20Object%20Reference) (OtherBodyIndex :type Integer) (bFromSweep :type Boolean) (SweepResult :type Hit%20Result%20Structure%20%28by%20ref%29))
  (bind _returnvalue (Game|GetPlayerCharacter 0))
  ;[1 1 1] Overlap Fist Capsule
  (if (== OtherActor _returnvalue)
    (if (== (Utilities|GetClass _returnvalue) 0)
      (CallFunction|DoDmg))))

(event OnComponentBeginOverlap(RightFist)
  (params (OverlappedComponent :type Primitive%20Component%20Object%20Reference) (OtherActor :type Actor%20Object%20Reference) (OtherComp :type Primitive%20Component%20Object%20Reference) (OtherBodyIndex :type Integer) (bFromSweep :type Boolean) (SweepResult :type Hit%20Result%20Structure%20%28by%20ref%29))
  (bind _returnvalue (Game|GetPlayerCharacter 0))
  ;[1 1 1] Overlap Fist Capsule
  (if (== OtherActor _returnvalue)
    (if (== (Utilities|GetClass _returnvalue) 0)
      (CallFunction|DoDmg))))

(event Custom|SeekPlayer
  ;[1 1 1] Initialisation Seeker Loop
  (if (Variables|Default|GetAlive)
    (if (not (Variables|Default|GetBlesse))
      (if (Variables|Default|GetisAttacking)
        (Components|Movement|StopMovementImmediately (Variables|Character|GetCharacterMovement))
        (else
          (AI|AIMoveTo self "0, 0, 0" (Game|GetPlayerCharacter 0) 1.5e+02 false
            (:then
              _)
            (:OnSuccess
              _)
            (:OnFail
              _))
          (Utilities|FlowControl|Delay 0.2)
          (CallFunction|SeekPlayer))))))

(event Custom|DistancePlayer
  ;[1 1 1] Player distance fonction
  (if (Variables|Default|GetAlive)
    (if (not (Variables|Default|GetBlesse))
      (Utilities|Time|SetTimerbyFunctionName 0 "PlayerDistance" 1.0 true))))

(event Custom|eColRightFist
  ;[1 1 1] Fist collision e/d
  (Collision|SetCollisionEnabled (Variables|Default|GetRightFist) "QueryAndPhysics"))

(event Custom|R_Trace
  (bind _rightfist (Variables|Default|GetRightFist))
  (bind _returnvalue (Transformation|GetWorldLocation _rightfist))
  ;[1 1 1] Fist Trace
  (bind _outhit (Collision|SphereTraceForObjects _returnvalue (+ _returnvalue (* (Math|Vector|GetForwardVector (Transformation|GetWorldRotation _rightfist)) 5e+01)) 64.0 (Utilities|Array|MakeArray "ObjectTypeQuery3") false 0 "ForDuration"))
  (if (== (.HitActor (Collision|BreakHitResult _outhit)) (Game|GetPlayerCharacter 0))
    (bind _returnvalue_2 (Effects|SpawnEmitteratLocation "/Game/StarterContent/Particles/P_FistSprite.P_FistSprite" (.Location (Collision|BreakHitResult _outhit))))
    (Transformation|SetWorldScale3D _returnvalue_2 "0.400000,0.400000,0.400000")
    (CallFunction|DoDmg)))

(event Custom|DoDmg
  ;[1 1 1] Damage
  (Game|Damage|ApplyDamage (Game|GetPlayerCharacter 0) (Math|Random|RandomFloatinRange (Variables|Default|GetMinDmg) (Variables|Default|GetMaxDmg)) 0 self))

(event Custom|Attack
  (Variables|Default|SetisAttacking true)
  (switch int (Math|Random|RandomIntegerinRange 0 3)
    (:0
      (Variables|Default|SetAttMontage "/Game/IA/AnimeMontageIA/Attack1.Attack1")
      (Variables|Default|SetMinDmg 0.0)
      (Variables|Default|SetMaxDmg 0.0))
    (:1
      (Variables|Default|SetAttMontage "/Game/IA/AnimeMontageIA/Attack2.Attack2")
      (Variables|Default|SetMinDmg 0.0)
      (Variables|Default|SetMaxDmg 0.0))
    (:2
      (Variables|Default|SetAttMontage "/Game/IA/AnimeMontageIA/Attack3.Attack3")
      (Variables|Default|SetMinDmg 0.0)
      (Variables|Default|SetMaxDmg 0.0))
    (:3
      (Variables|Default|SetAttMontage "/Game/IA/AnimeMontageIA/Attack4.Attack4")
      (Variables|Default|SetMinDmg 0.0)
      (Variables|Default|SetMaxDmg 0.0)))
  (bind _returnvalue (Animation|PlayAnimMontage (Variables|Default|GetAttMontage) 1.0 "None"))
  (Utilities|FlowControl|Delay _returnvalue)
  (Variables|Default|SetisAttacking false)
  (CallFunction|SeekPlayer)
  (if (<= (Variables|Default|GetDistance) 1e+02)
    (CallFunction|FacePlayer)))

(event Custom|dColRightFist
  ;[1 1 1] Fist collision e/d
  (Collision|SetCollisionEnabled (Variables|Default|GetRightFist) "NoCollision"))

(event Custom|L_Trace
  (bind _leftfist (Variables|Default|GetLeftFist))
  (bind _returnvalue (Transformation|GetWorldLocation _leftfist))
  ;[1 1 1] Fist Trace
  (bind _outhit (Collision|SphereTraceForObjects _returnvalue (+ _returnvalue (* (Math|Vector|GetForwardVector (Transformation|GetWorldRotation _leftfist)) 5e+01)) 64.0 (Utilities|Array|MakeArray "ObjectTypeQuery3") false 0 "ForDuration"))
  (if (== (.HitActor (Collision|BreakHitResult _outhit)) (Game|GetPlayerCharacter 0))
    (bind _returnvalue_2 (Effects|SpawnEmitteratLocation "/Game/StarterContent/Particles/P_FistSprite.P_FistSprite" (.Location (Collision|BreakHitResult _outhit))))
    (Transformation|SetWorldScale3D _returnvalue_2 "0.400000,0.400000,0.400000")
    (CallFunction|DoDmg)))

(event Custom|FacePlayer
  ;[1 1 1] FacePlayer
  (Transformation|SetActorRotation (Math|Rotator|FindLookatRotation (Transformation|GetActorLocation) (Transformation|GetActorLocation (Game|GetPlayerCharacter 0)))))

(event Custom|eColLeftFist
  ;[1 1 1] Fist collision e/d
  (Collision|SetCollisionEnabled (Variables|Default|GetLeftFist) "QueryAndPhysics"))

(event Custom|dColLeftFist
  ;[1 1 1] Fist collision e/d
  (Collision|SetCollisionEnabled (Variables|Default|GetLeftFist) "NoCollision"))

(event Game|Damage|EventAnyDamage
  (params (Damage :type Float%20%28single-precision%29) (DamageType :type Damage%20Type%20Object%20Reference) (InstigatedBy :type Controller%20Object%20Reference) (DamageCauser :type Actor%20Object%20Reference))
  ;[1 1 1] Get Damage
  (if (!= DamageCauser self)
    (Variables|Default|SetDamage Damage)
    (bind _output_get (Variables|Default|SetHealth (- (Variables|Default|GetHealth) (/ Damage (Variables|Default|GetArmor)))))
    (if (<= _output_get 0.0)
      (Utilities|FlowControl|DoOnce false :!label _label
        (:Completed
          (Animation|PlayAnimMontage "/Game/IA/AnimeMontageIA/KO.KO" 1.0 "None")
          (Variables|Default|SetAlive false)))
      (elif (>= (Variables|Default|GetDamage) 5.0)
        (Variables|Default|SetBlesse true)
        (bind _returnvalue (Animation|PlayAnimMontage "/Game/IA/AnimeMontageIA/Blesse.Blesse" 1.0 "None"))
        (Utilities|FlowControl|Delay _returnvalue)
        (Variables|Default|SetBlesse false)
        (if (<= (Variables|Default|GetHealth) 0.0)
          (goto _label))))))

(event EventBeginPlay
  ;[1 1 1] Initialisation IA
  (Variables|Default|SetAlive true)
  (Utilities|FlowControl|Delay 0.2)
  (CallFunction|SeekPlayer)
  (CallFunction|DistancePlayer)
  (Variables|Default|SetHealth 1e+03)
  (Variables|Default|SetArmor 1.0)
  (bind _returnvalue (UserInterface|CreateWidget "/Game/Menu/IAHB.IAHB_C"))
  (UserInterface|Viewport|AddtoViewport _returnvalue 0))

(event EventTick
  (params (DeltaSeconds :type Float%20%28single-precision%29))
  (AI|AIMoveTo self "0, 0, 0" (Game|GetPlayerCharacter 0) 5e+01 false))

(fn ConstructionScript)

(fn PlayerDistance
  (if (not (Variables|Default|GetisAttacking))
    ;[1 1 1] Detect player
    (bind _output_get (Variables|Default|SetDistance (Math|Vector|VectorLength (- (Transformation|GetActorLocation) (Transformation|GetActorLocation (Game|GetPlayerCharacter 0))))))
    ;[1 1 1] Attack
    (if (<= _output_get 1e+02)
      (CallFunction|Attack))))